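; Base weapon Blueprint for the FPS player's guns, handling firing, recoil, ammo, reload math and typed ammo pickups.
; StartShooting spends a round, auto-reloads when empty, then either line-traces from the camera (looped for shotgun pellets, random spread unless aiming) or spawns an optionally homing projectile from the weapon socket.
; Hits apply damage through interface messages and report AI damage events.
; A timeline drives recoil as controller pitch and yaw, then reverses.
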(event Custom|AutoReloadOnEmpty
  ;[0.07198 0.09896 0.07803] Automatically calls reload event
  (if (Utilities|Enum|Equal(Enum) (Variables|weapopndata|GetWeaponType) "NewEnumerator3") ; Sniper cause issue if reloading happens after the last bullet is fired
    (Utilities|FlowControl|Delay 0.3)
    (Default|Reload (Variables|Default|GetPlayer))
    (CallFunction|WeaponAimExit)
    (else
      (Default|Reload (Variables|Default|GetPlayer)))))

(event Custom|StartRecoil
  (bind _returnvalue (Game|GetPlayerCharacter 0))
  ;[0.2348 0.25 0] Adds recoil effect to weapons
  (bind (_direction _alpha) (Timeline|Recoil PlayFromStart)
    (:Update
      (switch Utilities|FlowControl|Switch|SwitchonETimelineDirection _direction
        (:Forward
          (Pawn|Input|AddControllerPitchInput _returnvalue (Math|Float|Lerp 0.0 (Variables|WeapopnData|GetWeaponKick) _alpha))
          (Pawn|Input|AddControllerYawInput (Game|GetPlayerCharacter 0) (Math|Random|RandomFloatinRange -0.15 0.15)))
        (:Backward
          (Pawn|Input|AddControllerPitchInput _returnvalue (* (Math|Float|Lerp 0.0 (Variables|WeapopnData|GetWeaponKick) _alpha) -1.0)))))
    (:Finished
      (CallFunction|ReverseRecoil)
      (Utilities|FlowControl|RetriggerableDelay 0.05)
      (CallFunction|StopRecoil))))

(event Custom|StopRecoil
  (bind _returnvalue (Game|GetPlayerCharacter 0))
  ;[0.2348 0.25 0] Adds recoil effect to weapons
  (bind (_direction _alpha) (Timeline|Recoil Stop)
    (:Update
      (switch Utilities|FlowControl|Switch|SwitchonETimelineDirection _direction
        (:Forward
          (Pawn|Input|AddControllerPitchInput _returnvalue (Math|Float|Lerp 0.0 (Variables|WeapopnData|GetWeaponKick) _alpha))
          (Pawn|Input|AddControllerYawInput (Game|GetPlayerCharacter 0) (Math|Random|RandomFloatinRange -0.15 0.15)))
        (:Backward
          (Pawn|Input|AddControllerPitchInput _returnvalue (* (Math|Float|Lerp 0.0 (Variables|WeapopnData|GetWeaponKick) _alpha) -1.0)))))
    (:Finished
      (CallFunction|ReverseRecoil)
      (Utilities|FlowControl|RetriggerableDelay 0.05)
      (CallFunction|StopRecoil))))

(event Custom|ReverseRecoil
  (bind _returnvalue (Game|GetPlayerCharacter 0))
  ;[0.2348 0.25 0] Adds recoil effect to weapons
  (bind (_direction _alpha) (Timeline|Recoil Reverse)
    (:Update
      (switch Utilities|FlowControl|Switch|SwitchonETimelineDirection _direction
        (:Forward
          (Pawn|Input|AddControllerPitchInput _returnvalue (Math|Float|Lerp 0.0 (Variables|WeapopnData|GetWeaponKick) _alpha))
          (Pawn|Input|AddControllerYawInput (Game|GetPlayerCharacter 0) (Math|Random|RandomFloatinRange -0.15 0.15)))
        (:Backward
          (Pawn|Input|AddControllerPitchInput _returnvalue (* (Math|Float|Lerp 0.0 (Variables|WeapopnData|GetWeaponKick) _alpha) -1.0)))))
    (:Finished
      (CallFunction|ReverseRecoil)
      (Utilities|FlowControl|RetriggerableDelay 0.05)
      (CallFunction|StopRecoil))))

(event Custom|FireRateCalculate
  ;[0.09082 0.2135 0.1185] Fire rate for non-automatic weapons
  (Variables|/Game/FPSGame/_PlayerCharacter/BP_Player.BP_Player_C|SetIsWeaponFireLoading? (Variables|Default|GetPlayer) true)
  (Utilities|FlowControl|Delay (Variables|WeapopnData|GetFireRate))
  (Variables|/Game/FPSGame/_PlayerCharacter/BP_Player.BP_Player_C|SetIsWeaponFireLoading? (Variables|Default|GetPlayer) false))

(event Custom|WeaponAimEnter
  ;[0 0.07392 0.349] Binds aiming bool to ADS input action on BP_Player
  (Variables|Default|SetIsAimingWeapon? true))

(event Custom|WeaponAimExit
  ;[0 0.07392 0.349] Binds aiming bool to ADS input action on BP_Player
  (Variables|Default|SetIsAimingWeapon? false))

(event Custom|GunRecoil
  (Utilities|FlowControl|DoOnce false :!label _label
    (:Completed
      (Animation|Montage|PlayMontage (Variables|/Game/FPSGame/_PlayerCharacter/BP_Player.BP_Player_C|GetPlayerArms (Variables|Default|GetPlayer)) "/Game/FPSGame/_PlayerCharacter/Animations_Retargeted/PlayerFPP_RifleAimFire_Montage.PlayerFPP_RifleAimFire_Montage"
        (:OnCompleted
          (goto _label Reset))))))

(event EventBeginPlay
  ;[0.07198 0.09896 0.07803] Get reference to Player
  (bind _asbp_player (Utilities|Casting|CastToBP_Player (Game|GetPlayerCharacter 0)))
  (bind _output_get (Variables|Default|SetPlayer _asbp_player))
  ;[0 0.07392 0.349] Binds aiming bool to ADS input action on BP_Player
  (EventDispatchers|BindEventtoAimEnter _output_get (delegate Custom|WeaponAimEnter))
  (EventDispatchers|BindEventtoAimExit _output_get (delegate Custom|WeaponAimExit)))

(event EventTick
  (params (DeltaSeconds :type Float%20%28single-precision%29))
  (Default|AimFieldOfView (Variables|Default|GetPlayer)))

(fn ConstructionScript)

(fn StartShooting
  (params (FireType :type E_FireTypes%20Enum :default "NewEnumerator0"))
  (bind _weaponstats (Variables|Default|GetWeaponStats))
  (bind _weaponmesh (Variables|Default|GetWeaponMesh))
  (bind _damage (Utilities|Struct|BreakS_WeaponStats _weaponstats))
  (bind _returnvalue (Components|GetOwner _weaponmesh))
  (Utilities|FlowControl|Sequence
    (:then_0
      ;[0.07198 0.09896 0.07803] Subtracts one bullet when firing weapon
      (Variables|Ammodata|SetCurrentAmmo (- (Variables|Ammodata|GetCurrentAmmo) 1))
      ;[0.008473 0.08959 0.125] Auto reload when mag empty
      (if (<= (Variables|Ammodata|GetCurrentAmmo) 0)
        (CallFunction|AutoReloadonEmpty)))
    (:then_1
      (switch Utilities|FlowControl|Switch|SwitchonE_FireTypes FireType
        (:NewEnumerator0
          (if (Variables|ShotGun|GetIsShotgun)
            ;[0.05084 0.01528 0.0625] Shoots extra line traces for shot gun pellets
            (for _index (range 0 (- (Variables|ShotGun|GetPelletCount) 1))
              ;[0.1038 0.07003 0.1719] Draws line trace for hitscan weapons
              (bind _hitresult (CallFunction|CalculateLineTrace (Variables|/Game/FPSGame/_PlayerCharacter/BP_Player.BP_Player_C|GetCamera (Variables|Default|GetPlayer))))
              (CallFunction|AddDamage _hitresult)
              (Game|SpawnActorfromClass (Variables|Default|GetImpactEffect) (Math|Transform|MakeTransform (.ImpactPoint (Collision|BreakHitResult _hitresult)) "0, 0, 0" "1,1,1") "Undefined" 0 _hitresult 0)
              (CallFunction|StartRecoil)
              (CallFunction|GunRecoil)
              (Variables|WeapopnData|SetIsFiring? true)
              (Class|BPIDamageble|TakeDamageBPID(Message) (.HitActor (Collision|BreakHitResult _hitresult)) (Utilities|Struct|MakeS_DamageInfo _damage "NewEnumerator0" "NewEnumerator1" false true) _returnvalue)
              (Class|AISenseDamage|ReportDamageEvent (.HitActor (Collision|BreakHitResult _hitresult)) self _damage (Transformation|GetActorLocation _returnvalue) (.Location (Collision|BreakHitResult _hitresult)) "None"))
            (else
              (bind _hitresult_2 (CallFunction|CalculateLineTrace (Variables|/Game/FPSGame/_PlayerCharacter/BP_Player.BP_Player_C|GetCamera (Variables|Default|GetPlayer))))
              (CallFunction|AddDamage _hitresult_2)
              (Game|SpawnActorfromClass (Variables|Default|GetImpactEffect) (Math|Transform|MakeTransform (.ImpactPoint (Collision|BreakHitResult _hitresult_2)) "0, 0, 0" "1,1,1") "Undefined" 0 _hitresult_2 0)
              (CallFunction|StartRecoil :!label _label)
              (CallFunction|GunRecoil)
              (Variables|WeapopnData|SetIsFiring? true)
              (Class|BPIDamageble|TakeDamageBPID(Message) (.HitActor (Collision|BreakHitResult _hitresult_2)) (Utilities|Struct|MakeS_DamageInfo _damage "NewEnumerator0" "NewEnumerator1" false true) _returnvalue)
              (Class|AISenseDamage|ReportDamageEvent (.HitActor (Collision|BreakHitResult _hitresult_2)) self _damage (Transformation|GetActorLocation _returnvalue) (.Location (Collision|BreakHitResult _hitresult_2)) "None"))))
        (:NewEnumerator1
          ;[0.03909 0.09375 0.05605] Spawns projectile
          (bind _projectiletransform (CallFunction|CalculateProjectile (Variables|/Game/FPSGame/_PlayerCharacter/BP_Player.BP_Player_C|GetCamera (Variables|Default|GetPlayer)) (Variables|Default|GetWeaponMesh) (Variables|Default|GetWeaponSocket)))
          (Game|SpawnActorfromClass (Variables|Default|GetProjectile) _projectiletransform "Undefined" 0 (Variables|Default|GetWeaponStats) "1.000000,0.000000,0.000000" (Variables|Default|GetHomingMissile?) 0)
          (goto _label))))))

(fn CalculateLineTrace
  (params (Camera :type Camera%20Component%20Object%20Reference))
  (bind _bulletspread (Variables|weapopndata|GetBulletSpread))
  (bind _returnvalue (* _bulletspread -1.0))
  (Utilities|FlowControl|Sequence
    (:then_0
      (LocalVariables|SetLocalCamera Camera))
    (:then_1
      (bind _outhit (Collision|LineTraceForObjects (.location (Transformation|GetWorldTransform (LocalVariables|GetLocalCamera))) (select (Variables|/Game/FPSGame/_PlayerCharacter/BP_Player.BP_Player_C|GetIsAiming? (Variables|Default|GetPlayer)) (+ (.location (Transformation|GetWorldTransform (LocalVariables|GetLocalCamera))) (* (Math|Vector|GetForwardVector (.rotation (Transformation|GetWorldTransform (LocalVariables|GetLocalCamera)))) (Variables|WeapopnData|GetHit%20Distance))) (Math|Vector|MakeVector (+ (.X (Math|Vector|BreakVector (+ (.location (Transformation|GetWorldTransform (LocalVariables|GetLocalCamera))) (* (Math|Vector|GetForwardVector (.rotation (Transformation|GetWorldTransform (LocalVariables|GetLocalCamera)))) (Variables|WeapopnData|GetHit%20Distance))))) (Math|Random|RandomFloatinRange _returnvalue _bulletspread)) (+ (.Y (Math|Vector|BreakVector (+ (.location (Transformation|GetWorldTransform (LocalVariables|GetLocalCamera))) (* (Math|Vector|GetForwardVector (.rotation (Transformation|GetWorldTransform (LocalVariables|GetLocalCamera)))) (Variables|WeapopnData|GetHit%20Distance))))) (Math|Random|RandomFloatinRange _returnvalue _bulletspread)) (+ (.Z (Math|Vector|BreakVector (+ (.location (Transformation|GetWorldTransform (LocalVariables|GetLocalCamera))) (* (Math|Vector|GetForwardVector (.rotation (Transformation|GetWorldTransform (LocalVariables|GetLocalCamera)))) (Variables|WeapopnData|GetHit%20Distance))))) (Math|Random|RandomFloatinRange _returnvalue _bulletspread)))) (Utilities|Array|MakeArray "ObjectTypeQuery1" "ObjectTypeQuery2" "ObjectTypeQuery3") false (Utilities|Array|MakeArray (Game|GetPlayerCharacter 0)) "None" true "(R=1.000000,G=0.000000,B=0.000000,A=1.000000)" "(R=0.000000,G=1.000000,B=0.000000,A=1.000000)" 1e+01)))
    (:then_2
      (return _outhit))))

(fn ReloadCalculation
  (bind _output_get (Variables|AmmoData|SetBulletDifference (- (Variables|AmmoData|GetMagazineSize) (Variables|Ammodata|GetCurrentAmmo))))
  (if (<= _output_get (Variables|AmmoData|GetTotalAmmo))
    ;[0.05458 0.05779 0.1302] Runs when there is reserve ammo
    (Variables|Ammodata|SetCurrentAmmo (Variables|AmmoData|GetMagazineSize))
    (Variables|AmmoData|SetTotalAmmo (- (Variables|AmmoData|GetTotalAmmo) (Variables|AmmoData|GetBulletDifference)))
    (else
      ;[0.05458 0.05779 0.1302] Runs when reserve amount is lower than ammo in magazine
      (Variables|Ammodata|SetCurrentAmmo (+ (Variables|Ammodata|GetCurrentAmmo) (Variables|AmmoData|GetTotalAmmo)))
      (Variables|AmmoData|SetTotalAmmo 0))))

(fn AmmoPickup
  (params (AmmoType :type E_AmmoType%20Enum :default "NewEnumerator0"))
  (switch Utilities|FlowControl|Switch|SwitchonE_AmmoType AmmoType
    (:NewEnumerator0
      ;[0 0.2488 0.5] Adds ammo to Pistol if picked up by Pistol
      (if (Utilities|Enum|Equal(Enum) (Variables|weapopndata|GetWeaponType) "NewEnumerator0")
        (Variables|AmmoData|SetTotalAmmo (+ (Variables|Ammo|GetPistolPickupAmount) (Variables|AmmoData|GetTotalAmmo)))
        (return true)
        (else
          (return false))))
    (:NewEnumerator1
      ;[0 0.2488 0.5] Adds ammo to AutoRifle if picked up by AutoRifle
      (if (Utilities|Enum|Equal(Enum) (Variables|weapopndata|GetWeaponType) "NewEnumerator1")
        (Variables|AmmoData|SetTotalAmmo (+ (Variables|Ammo|GetAutoRiflePickupAmount) (Variables|AmmoData|GetTotalAmmo)))
        (return true)
        (else
          (return false))))
    (:NewEnumerator2
      ;[0 0.2488 0.5] Adds ammo to Shotgun if picked up by Shotgun
      (if (Utilities|Enum|Equal(Enum) (Variables|weapopndata|GetWeaponType) "NewEnumerator2")
        (Variables|AmmoData|SetTotalAmmo (+ (Variables|Ammo|GetShotgunPickupAmount) (Variables|AmmoData|GetTotalAmmo)))
        (return true)
        (else
          (return false))))
    (:NewEnumerator3
      ;[0 0.2488 0.5] Adds ammo to SniperRifle if picked up by SniperRifle
      (if (Utilities|Enum|Equal(Enum) (Variables|weapopndata|GetWeaponType) "NewEnumerator3")
        (Variables|AmmoData|SetTotalAmmo (+ (Variables|Ammo|GetSniperRiflePickupAmount) (Variables|AmmoData|GetTotalAmmo)))
        (return true)
        (else
          (return false))))
    (:NewEnumerator4
      ;[0 0.2488 0.5] Adds ammo to GrenadeLauncher if picked up by GrenadeLauncher
      (if (Utilities|Enum|Equal(Enum) (Variables|weapopndata|GetWeaponType) "NewEnumerator4")
        (Variables|AmmoData|SetTotalAmmo (+ (Variables|Ammo|GetGrenadeLauncherPickupAmount) (Variables|AmmoData|GetTotalAmmo)))
        (return true)
        (else
          (return false))))
    (:NewEnumerator5
      ;[0 0.2488 0.5] Adds ammo to RocketLauncher if picked up by RocketLauncher
      (if (Utilities|Enum|Equal(Enum) (Variables|weapopndata|GetWeaponType) "NewEnumerator5")
        (Variables|AmmoData|SetTotalAmmo (+ (Variables|Ammo|GetRocketLauncherPickupAmount) (Variables|AmmoData|GetTotalAmmo)))
        (return true)
        (else
          (return false))))))

(fn IsMagFullorEmpty?
  (if (== (Variables|Ammodata|GetCurrentAmmo) (Variables|AmmoData|GetMagazineSize))
    _
    (elif (== (Variables|AmmoData|GetTotalAmmo) 0)
      _
      (else
        ;[0.224 0.1508 0.1306] Enables reload if magazine is empty but ammo available in reserve
        (bind _output_get (Variables|/Game/FPSGame/_PlayerCharacter/BP_Player.BP_Player_C|SetCanReload? (Variables|Default|GetPlayer) true))
        (return _output_get))))
  ;[0.224 0.1508 0.1306] Disables reload if magazine is full or reserves are empty
  (bind _output_get_2 (Variables|/Game/FPSGame/_PlayerCharacter/BP_Player.BP_Player_C|SetCanReload? (Variables|Default|GetPlayer) false))
  (return _output_get_2))

(fn DoWeHaveAmmo?
  ;[0.04281 0.1719 0.03416] Allow shooting if player has ammo
  (return (> (Variables|Ammodata|GetCurrentAmmo) 0)))

(fn IsThereAmmoLeft?
  ;[0.04281 0.1719 0.03416] Checks to see if there is ammo in reserves
  (return (> (Variables|AmmoData|GetTotalAmmo) 0)))

(fn StopShooting
  ;[0.05458 0.05779 0.1302] Se IsFiring? to false
  (Variables|WeapopnData|SetIsFiring? false))

(fn ShotgunReloadPellets
  (Variables|WeapopnData|SetReloadTime (* (- (Variables|AmmoData|GetMagazineSize) (Variables|Ammodata|GetCurrentAmmo)) (Variables|WeapopnData|GetReloadTime))))

(fn AddDamage
  (params (HitResult :type Hit%20Result%20Structure))
  ;[0.03993 0.0479 0.1042] Passes info thru weapon to enemy taking damage
  (Class|BPITakeDamage|EnemyTakeDamage(Message) (.HitActor (Collision|BreakHitResult HitResult)) (Variables|Default|GetWeaponStats) HitResult))

(fn CalculateProjectile
  (params (Camera :type Camera%20Component%20Object%20Reference) (WeaponMesh :type Scene%20Component%20Object%20Reference) (WeaponSocket :type Name))
  (Utilities|FlowControl|Sequence
    (:then_0
      (LocalVariables|SetLocalCamera Camera)
      (LocalVariables|SetLocalWeaponMesh WeaponMesh)
      (LocalVariables|SetLocalWeaponSocket WeaponSocket))
    (:then_1
      ;[0.1615 0.0204 0.1398] Gets player camera rotation and location of equipped weapon socket
      (LocalVariables|SetLocalProjectileTransfom (Math|Transform|MakeTransform (Transformation|GetSocketLocation (LocalVariables|GetLocalWeaponMesh) (LocalVariables|GetLocalWeaponSocket)) (Pawn|GetControlRotation (.AsBP%20Player (Utilities|Casting|CastToBP_Player (Components|GetOwner (LocalVariables|GetLocalCamera)))) :!class /Script/Engine.Pawn))))
    (:then_2
      (return (LocalVariables|GetLocalProjectileTransfom)))))